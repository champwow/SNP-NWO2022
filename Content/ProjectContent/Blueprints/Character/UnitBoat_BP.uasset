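; UnitBoat_BP is a selectable RTS boat unit that toggles a selection decal and joins or leaves the controller's selection when left-clicked by the BLUE side.
; A move stops active movement, then a timeline glides the capsule along the mesh's reversed forward vector while lerping yaw toward the blackboard TargetLocation.
; On finish it asks UnitAIController to run the server move.
; It also spawns a RotateMeasure actor at the destination, facing the boat.
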(event Custom|IsSelected
  (params (IsSelected :type Boolean))
  ;[1 1 1] If AI Selected it will Visibility
  (Rendering|SetVisibility (Variables|Default|GetDecal) IsSelected false))

(event Custom|CreateLine
  ;[1 1 1] Create Line for Measure Forward Actor BT Boat and Rotate Measure
  (if (Utilities|IsValid (Variables|Default|GetRotateMeasure))
    (Actor|DestroyActor (Variables|Default|GetRotateMeasure)))
  (bind _returnvalue (Game|SpawnActorfromClass "/Game/ProjectContent/Blueprints/Character/RotateMeasure_BP.RotateMeasure_BP_C" (Math|Transform|MakeTransform (Variables|Default|GetDestinationLocation) "0, 0, 0" "1,1,1") "Undefined" 0 0))
  (Variables|Default|SetRotateMeasure _returnvalue)
  (Transformation|SetWorldRotation (Variables|/Script/Engine.Actor|GetRootComponent _returnvalue) (Math|Rotator|MakeRotator (.roll (Math|Rotator|FindLookatRotation (Transformation|GetWorldLocation (Variables|/Script/Engine.Actor|GetRootComponent _returnvalue)) (Transformation|GetActorLocation))) (.pitch (Math|Rotator|FindLookatRotation (Transformation|GetWorldLocation (Variables|/Script/Engine.Actor|GetRootComponent _returnvalue)) (Transformation|GetActorLocation))) (.yaw (Math|Rotator|FindLookatRotation (Transformation|GetWorldLocation (Variables|/Script/Engine.Actor|GetRootComponent _returnvalue)) (Transformation|GetActorLocation)))) false false))

(event Custom|AIMoveToLocation
  (bind _self self)
  ;[1 1 1] AI MoveTo on Server Side
  (AI|AIMoveTo _self (AI|Components|Blackboard|GetValueasVector (AI|GetBlackboard _self) (Utilities|Name|MakeLiteralName "TargetLocation")) 0 5.0 false))

(event Custom|MoveToLocation
  (bind _capsulecomponent (Variables|Collision|GetCapsuleComponent))
  (bind _returnvalue (Transformation|GetWorldRotation _capsulecomponent))
  ;[1 1 1] AI Rotate and Move Forward Following Forward Vector
  (Utilities|FlowControl|Sequence
    (:then_0
      (Components|Timeline|SetPlayRate (Variables|Default|GetRotateToLocation) 1.0)
      (bind _newtrack_0 (Timeline|RotateToLocation PlayFromStart)
        (:Update
          (Transformation|SetWorldLocation (Variables|Collision|GetCapsuleComponent) (+ (Transformation|GetWorldLocation (Variables|Collision|GetCapsuleComponent)) (* (* (* (Math|Vector|GetForwardVector (Variables|Character|GetMesh)) "-1.000000,-1.000000, 0") 1e+02) (Utilities|Time|GetWorldDeltaSeconds))) false false)
          (Transformation|SetWorldRotation (Variables|Collision|GetCapsuleComponent) (Math|Rotator|Lerp(Rotator) (Math|Rotator|MakeRotator (.roll _returnvalue) (.pitch _returnvalue) (.yaw _returnvalue)) (Math|Rotator|MakeRotator (.roll _returnvalue) (.pitch _returnvalue) (.yaw (Math|Rotator|FindLookatRotation (Transformation|GetWorldLocation _capsulecomponent) (AI|Components|Blackboard|GetValueasVector (AI|GetBlackboard self) (Utilities|Name|MakeLiteralName "TargetLocation"))))) (/ _newtrack_0 3e+01) true) false false))
        (:Finished
          (Variables|Default|SetCheckFirst? false)
          (bind _asunit_aicontroller (Utilities|Casting|CastToUnitAIController (AI|GetAIController self)))
          (Default|AIMovetoonServer _asunit_aicontroller))))
    (:then_1
      (if (not (Variables|Default|GetCheckFirst?))
        (Class|NavMovementComponent|StopActiveMovement (Variables|Character|GetCharacterMovement))))))

(event EventBeginPlay
  (Networking|ForceNetUpdate))

(event MouseInput|EventActorOnClicked
  (params (ButtonPressed :type Key%20Structure :default "None"))
  (bind _asrtsgame_instance (Utilities|Casting|CastToRTSGameInstance (Game|GetGameInstance)))
  ;[1 1 1] When Actor OnClicked It will Visible / Hidden Decal and Add / Remove Unit from Selection Array
  (if (Utilities|Enum|Equal(Enum) (Variables|/Game/ProjectContent/Blueprints/RTSGameInstance.RTSGameInstance_C|GetUserSide _asrtsgame_instance) "BLUE")
    (if (== ButtonPressed "LeftMouseButton")
      (bind _asrtscontroller (Utilities|Casting|CastToRTSController (Game|GetPlayerController 0)))
      (if (Rendering|IsVisible (Variables|Default|GetDecal))
        (Default|RemovUnitfromSelection _asrtscontroller self)
        (else
          (Default|AddUnittoSelection _asrtscontroller self))))))

(fn ConstructionScript)